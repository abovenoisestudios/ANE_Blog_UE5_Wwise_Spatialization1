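; Sound source actor that plays as a Wwise multi-position emitter, set up on BeginPlay.
; A Blueprint flag selects either the Blueprint function or SetFiveSoundPositions, both given the same offsets.
; The Blueprint function builds five transforms along world Y, centred on the actor and mirrored either side, keeping its rotation and scale.
; It passes them to the AkComponent through SetMultiplePositions in MultiSources mode.
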(event EventBeginPlay
  ;[0.7531 0.1852 1] Set Multi-Position sound on Event Begin Play
  (if (Variables|Default|GetbBlueprint)
    (CallFunction|BPFSetFiveSoundPositions 6.5e+02 1.3e+03)
    (else
      (Class|SoundSourceActor|SetFiveSoundPositions 6.5e+02 1.3e+03))))

(fn ConstructionScript
  (|CallParentFunction))

(fn BPFSetFiveSoundPositions
  (params (OffsetY1 :type Float%20%28double-precision%29) (OffsetY2 :type Float%20%28double-precision%29))
  (bind _returnvalue (Transformation|GetActorTransform))
  (bind (_location _rotation _scale) (Math|Transform|BreakTransform _returnvalue))
  ;[1 0.7038 0.05542] Set Five Sound Positions
  (Utilities|FlowControl|Sequence
    (:then_0
      (LocalVariables|SetOffsetsArray (Utilities|Array|MakeArray 0.0 OffsetY1 OffsetY2 (* OffsetY1 -1.0) (* OffsetY2 -1.0))))
    (:then_1
      (for _array_element (LocalVariables|GetOffsetsArray)
        (Utilities|Array|Add (LocalVariables|GetPositionsArray) (Math|Transform|MakeTransform (Math|Vector|MakeVector (.x _location) (+ _array_element (.y _location)) (.z _location)) _rotation _scale)))
      (Class|AkGameplayStatics|SetMultiplePositions (Variables|Default|GetAkComponent) (LocalVariables|GetPositionsArray) "MultiSources"))))