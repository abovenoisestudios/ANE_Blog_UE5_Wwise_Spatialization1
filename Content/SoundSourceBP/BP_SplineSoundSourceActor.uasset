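; A spline sound source actor that keeps its Wwise AkComponent at the point on the spline nearest the player character.
; Each tick, a Blueprint flag selects either the local BPF follow function or SplineFollowPlayerCharacter, whose body is not in this graph.
; The Blueprint version moves the emitter to that closest point, or prints a warning if the spline is inactive.
; The construction script sets the spline component to auto-activate.
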(event EventTick
  (params (DeltaSeconds :type Float%20%28single-precision%29))
  ;[0.06419 1 0.9872] Follow the Player's Character on Event Tick
  (if (Variables|Default|GetbBlueprint)
    (CallFunction|BPFSplineFollowPlayerCharacter)
    (else
      (Class|SoundSourceActor|SplineFollowPlayerCharacter))))

(fn ConstructionScript
  ;[0.1335 0.3754 1] Activate the spline component on this class constructor (BP_SplineSoundSourceActor)
  (|CallParentFunction)
  (Components|Activation|SetAutoActivate (Variables|Default|GetSplineComponent) true))

(fn BPFSplineFollowPlayerCharacter
  ;[1 0.2675 0.01243] Spline Follow Player Character
  (if (Components|Activation|IsActive (Variables|Default|GetSplineComponent))
    (Transformation|SetWorldLocation (Variables|Default|GetAkComponent) (Spline|FindLocationClosesttoWorldLocation (Variables|Default|GetSplineComponent) (Transformation|GetActorLocation (Variables|Default|GetPlayerCharacter)) "World") false false)
    (else
      (Development|PrintString "Spline Component is not active" true true "(R=1.000000,G=0.000000,B=0.019874,A=1.000000)" 1e+01 "3"))))