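; Wwise sound source actor that plays its Ak Component's event while the player character overlaps its sphere and stops it on exit.
; A Blueprint flag routes both overlap events to either the local BPF_PlayAudioEvent function or a separate PlayAudioEvent implementation defined outside these graphs.
; The Blueprint version validates the audio event, optionally prints debug messages on play, and clears on-screen messages on stop.
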(event OnComponentBeginOverlap(SphereComponent)
  (params (OverlappedComponent :type Primitive%20Component%20Object%20Reference) (OtherActor :type Actor%20Object%20Reference) (OtherComp :type Primitive%20Component%20Object%20Reference) (OtherBodyIndex :type Integer) (bFromSweep :type Boolean) (SweepResult :type Hit%20Result%20Structure%20%28by%20ref%29))
  (bind _bdebug (Variables|Default|GetbDebug))
  (bind _debugmessage (Variables|Default|GetDebugMessage))
  ;[1 0.2691 0.07659] Plays Ak Component audio event on Begin Overlap
  (if (== OtherActor (Variables|Default|GetPlayerCharacter))
    (if (Variables|Audio|GetbBlueprint)
      (CallFunction|BPFPlayAudioEvent true _bdebug _debugmessage)
      (else
        (Class|SoundSourceActor|PlayAudioEvent true _bdebug _debugmessage)))))

(event OnComponentEndOverlap(SphereComponent)
  (params (OverlappedComponent :type Primitive%20Component%20Object%20Reference) (OtherActor :type Actor%20Object%20Reference) (OtherComp :type Primitive%20Component%20Object%20Reference) (OtherBodyIndex :type Integer))
  (bind _bdebug (Variables|Default|GetbDebug))
  (bind _debugmessage (Variables|Default|GetDebugMessage))
  ;[0.3055 0.3199 1] Stops Ak Component audio event on End Overlap
  (if (== OtherActor (Variables|Default|GetPlayerCharacter))
    (if (Variables|Audio|GetbBlueprint)
      (CallFunction|BPFPlayAudioEvent false _bdebug _debugmessage)
      (else
        (Class|SoundSourceActor|PlayAudioEvent false _bdebug _debugmessage)))))

(fn ConstructionScript)

(fn BPFPlayAudioEvent
  (params (bPlay :type Boolean) (bDebug :type Boolean) (_DebugMessage :type String))
  (bind _akcomponent (Variables|Default|GetAkComponent))
  ;[1 0.9104 0.4562] Play Audio Event
  (Utilities|FlowControl|Sequence
    (:then_0
      (LocalVariables|SetPlay bPlay)
      (LocalVariables|SetDebug bDebug))
    (:then_1
      (Utilities|IsValid (Variables|/Script/AkAudio.AkGameObject|GetAkAudioEvent (Variables|Default|GetAkComponent))
        (:Is%20Valid
          (if (LocalVariables|GetPlay)
            (Class|AkGameObject|PostAssociatedAkEvent _akcomponent)
            (if (LocalVariables|GetDebug)
              (Development|PrintString (Variables|Default|GetDebugMessage) true true "(R=0.124467,G=0.000000,B=1.000000,A=1.000000)" 6e+01 "1")
              (Development|PrintString "Blueprint Implementation" true true "(R=0.000000,G=0.660000,B=1.000000,A=1.000000)" 6e+01 "2"))
            (else
              (Class|AkGameObject|Stop _akcomponent)
              (Class|SoundSourceActor|ClearonScreenDebugMessages))))))))